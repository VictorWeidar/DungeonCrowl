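; BaseCharacter is a base character Blueprint that tracks health and a death state.
; CalculateHealth adds a signed delta to Health, then calls CalculateDead, which sets IsDead once Health reaches zero or below.
; A constant-true inner branch means IsDead is never set back to false here.
; The event graph and construction script are empty.
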(fn `CalculateDead`
  (if (<= (`self.Health`) 0.0)
    (if true
      (set `self.IsDead` true)
      (else
        (set `self.IsDead` false)))))

(fn `CalculateHealth`
  (params (Delta :type "Float (double-precision)"))
  (set `self.Health` (+ Delta (`self.Health`)))
  (`self.CalculateDead`))

(fn `UserConstructionScript`)